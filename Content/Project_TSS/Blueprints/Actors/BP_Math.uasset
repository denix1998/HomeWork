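; BP_Math is an actor Blueprint that runs two math operations on BeginPlay and prints the results, with no other gameplay logic.
; It multiplies vectors N1 and N2 component-wise into N and prints the X, Y and Z components through formatted text.
; It then loops over Array to accumulate a total in Sum and prints that total.
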(event EventBeginPlay
  (Variables|Default|SetN (* (Variables|Default|GetN1) (Variables|Default|GetN2)))
  (Development|PrintString (Utilities|String|ToString(Text) (Utilities|Text|FormatText "Product of vectors = x={x} 
                                        y={y} 
                                        z={z}" (.X (Math|Vector|BreakVector (Variables|Default|GetN))) (.Y (Math|Vector|BreakVector (Variables|Default|GetN))) (.Z (Math|Vector|BreakVector (Variables|Default|GetN))))) true true "(R=1.000000,G=0.000000,B=1.000000,A=1.000000)" 5.0)
  (Variables|Default|SetSum 0)
  (for _array_element (Variables|Default|GetArray)
    (Variables|Default|SetSum (+ _array_element (Variables|Default|GetSum))))
  (Development|PrintString (Utilities|String|ToString(Text) (Utilities|Text|FormatText "Sum of elemets = {Sum}" (Variables|Default|GetSum))) true true "(R=1.000000,G=1.000000,B=1.000000,A=1.000000)" 5.0))

(fn ConstructionScript)