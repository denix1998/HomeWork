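; BP_Trigger is a box trigger that reacts to BP_Toucher-Lift actors entering and leaving it.
; Both overlap events set IsActorEntered and feed one shared branch that turns the PointLight blue on entry and red on exit.
; Entry also increments and prints a touch count.
; Each branch prints the color name from its DT_Color row, while the light colors themselves are hardcoded.
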(event OnComponentBeginOverlap(Box)
  (params (OverlappedComponent :type Primitive%20Component%20Object%20Reference) (OtherActor :type Actor%20Object%20Reference) (OtherComp :type Primitive%20Component%20Object%20Reference) (OtherBodyIndex :type Integer) (bFromSweep :type Boolean) (SweepResult :type Hit%20Result%20Structure%20%28by%20ref%29))
  (Utilities|Casting|CastToBP_Toucher-Lift OtherActor)
  (Variables|Default|SetbIsActorEntered true)
  (if (Variables|Default|GetbIsActorEntered)
    (Rendering|Components|Light|SetLightColor (Variables|Default|GetPointLight) "(R=0.000000,G=0.000000,B=1.000000,A=1.000000)" true)
    (Variables|Default|SetCount (+ (Variables|Default|GetCount) 1))
    (Development|PrintString (Utilities|String|ToString(Text) (Utilities|Text|FormatText "You touched {Count} times" (Variables|Default|GetCount))) true true "(R=0.000000,G=1.000000,B=0.000000,A=1.000000)")
    (bind _returnvalue (Utilities|GetDataTableRow "/Game/Project_TSS/Blueprints/DT_Color.DT_Color" "Blue")
      (:then
        (Development|PrintString (Utilities|String|ToString(Text) (Utilities|Text|FormatText "Name Color: {Name}" (Utilities|Struct|BreakS_ColorGrade _returnvalue))) true true "(R=0.000000,G=0.000000,B=1.000000,A=1.000000)")))
    (else
      (Rendering|Components|Light|SetLightColor (Variables|Default|GetPointLight) "(R=1.000000,G=0.000000,B=0.000000,A=1.000000)" true)
      (bind _returnvalue_2 (Utilities|GetDataTableRow "/Game/Project_TSS/Blueprints/DT_Color.DT_Color" "Red")
        (:then
          (Development|PrintString (Utilities|String|ToString(Text) (Utilities|Text|FormatText "Name Color: {Name}" (Utilities|Struct|BreakS_ColorGrade _returnvalue_2))) true true "(R=1.000000,G=0.000000,B=0.000000,A=1.000000)"))))))

(event OnComponentEndOverlap(Box)
  (params (OverlappedComponent :type Primitive%20Component%20Object%20Reference) (OtherActor :type Actor%20Object%20Reference) (OtherComp :type Primitive%20Component%20Object%20Reference) (OtherBodyIndex :type Integer))
  (Utilities|Casting|CastToBP_Toucher-Lift OtherActor)
  (Variables|Default|SetbIsActorEntered false)
  (if (Variables|Default|GetbIsActorEntered)
    (Rendering|Components|Light|SetLightColor (Variables|Default|GetPointLight) "(R=0.000000,G=0.000000,B=1.000000,A=1.000000)" true)
    (Variables|Default|SetCount (+ (Variables|Default|GetCount) 1))
    (Development|PrintString (Utilities|String|ToString(Text) (Utilities|Text|FormatText "You touched {Count} times" (Variables|Default|GetCount))) true true "(R=0.000000,G=1.000000,B=0.000000,A=1.000000)")
    (bind _returnvalue (Utilities|GetDataTableRow "/Game/Project_TSS/Blueprints/DT_Color.DT_Color" "Blue")
      (:then
        (Development|PrintString (Utilities|String|ToString(Text) (Utilities|Text|FormatText "Name Color: {Name}" (Utilities|Struct|BreakS_ColorGrade _returnvalue))) true true "(R=0.000000,G=0.000000,B=1.000000,A=1.000000)")))
    (else
      (Rendering|Components|Light|SetLightColor (Variables|Default|GetPointLight) "(R=1.000000,G=0.000000,B=0.000000,A=1.000000)" true)
      (bind _returnvalue_2 (Utilities|GetDataTableRow "/Game/Project_TSS/Blueprints/DT_Color.DT_Color" "Red")
        (:then
          (Development|PrintString (Utilities|String|ToString(Text) (Utilities|Text|FormatText "Name Color: {Name}" (Utilities|Struct|BreakS_ColorGrade _returnvalue_2))) true true "(R=1.000000,G=0.000000,B=0.000000,A=1.000000)"))))))

(fn ConstructionScript)