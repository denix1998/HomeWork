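; BP_BaseCharacter is a base character Blueprint that prints item names and tests a simple health system through debug keys.
; BeginPlay prints each DT_Items row's name, and keys 1–4 pass fixed gains or losses to SetHealth.
; SetHealth applies and prints in-range changes, rejecting those above a hard-coded 100 or at/below zero.
; Its result feeds CharacterDead, which prints a death message for the at/below-zero case, leaving Health unchanged.
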(event EventBeginPlay
  (bind _outrownames (DataTable|GetDataTableRowNames "/Game/Project_TSS/Blueprints/DT_Items.DT_Items"))
  (for _array_element _outrownames
    (bind _returnvalue (Utilities|GetDataTableRow "/Game/Project_TSS/Blueprints/DT_Items.DT_Items" _array_element)
      (:then
        (Development|PrintString (Utilities|String|ToString(Name) (.Name (Utilities|Struct|BreakS_InventoryItem _returnvalue))))))))

(event Input|KeyboardEvents|1
  (params (Key :type Key%20Structure :default "None"))
  (:Pressed
    (bind _bisdead (CallFunction|SetHealth 1e+01))
    (CallFunction|CharacterDead _bisdead)))

(event Input|KeyboardEvents|4
  (params (Key :type Key%20Structure :default "None"))
  (:Pressed
    (bind _bisdead (CallFunction|SetHealth -5.0))
    (CallFunction|CharacterDead _bisdead)))

(event Input|KeyboardEvents|2
  (params (Key :type Key%20Structure :default "None"))
  (:Pressed
    (bind _bisdead (CallFunction|SetHealth -1e+01))
    (CallFunction|CharacterDead _bisdead)))

(event Input|KeyboardEvents|3
  (params (Key :type Key%20Structure :default "None"))
  (:Pressed
    (bind _bisdead (CallFunction|SetHealth 5.0))
    (CallFunction|CharacterDead _bisdead)))

(fn ConstructionScript)

(fn SetHealth
  (params (ChangeValue :type Float%20%28double-precision%29))
  (if (not (or (> (+ (Variables|Default|GetHealth) ChangeValue) 1e+02) (<= (+ (Variables|Default|GetHealth) ChangeValue) 0.0)))
    (Variables|Default|SetHealth (+ (Variables|Default|GetHealth) ChangeValue))
    (Development|PrintString (Utilities|String|ToString(Text) (Utilities|Text|FormatText "Current Health is {Health} / {MaxHealth}" (Variables|Default|GetHealth) (Variables|Default|GetMaxHealth))))
    (else
      (return (<= (+ (Variables|Default|GetHealth) ChangeValue) 0.0)))))

(fn CharacterDead
  (params (bIsDead :type Boolean))
  (if bIsDead
    (Development|PrintString "CHARACTER IS DEAD" true true "(R=1.000000,G=0.000704,B=0.000000,A=1.000000)")))