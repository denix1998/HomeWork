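; BP_Door0 is an interactable sliding door that shows a text prompt while the player character overlaps its Box component.
; The Interface event opens or closes it based on IsClosed, which is not updated in these graphs.
; The SwitchDoor timeline slides the Box along its relative X axis, playing forward to open and reversing to close.
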(event OnComponentBeginOverlap(Box)
  (params (OverlappedComponent :type Primitive%20Component%20Object%20Reference) (OtherActor :type Actor%20Object%20Reference) (OtherComp :type Primitive%20Component%20Object%20Reference) (OtherBodyIndex :type Integer) (bFromSweep :type Boolean) (SweepResult :type Hit%20Result%20Structure%20%28by%20ref%29))
  (if (== OtherActor (Game|GetPlayerCharacter 0))
    (Rendering|SetVisibility (Variables|Default|GetTextRender) true false)))

(event OnComponentEndOverlap(Box)
  (params (OverlappedComponent :type Primitive%20Component%20Object%20Reference) (OtherActor :type Actor%20Object%20Reference) (OtherComp :type Primitive%20Component%20Object%20Reference) (OtherBodyIndex :type Integer))
  (if (== OtherActor (Game|GetPlayerCharacter 0))
    (Rendering|SetVisibility (Variables|Default|GetTextRender) false false)))

(event Custom|OpenDoor
  (bind _alpha (Timeline|SwitchDoor Play)
    (:Update
      (Transformation|SetRelativeLocation (Variables|Default|GetBox) (Math|Vector|MakeVector (Math|Float|Lerp 0.0 2e+02 _alpha) 0.0 0.0) false false))))

(event Custom|CloseDoor
  (bind _alpha (Timeline|SwitchDoor Reverse)
    (:Update
      (Transformation|SetRelativeLocation (Variables|Default|GetBox) (Math|Vector|MakeVector (Math|Float|Lerp 0.0 2e+02 _alpha) 0.0 0.0) false false))))

(event EventInterface
  (params (Character :type Character%20Object%20Reference))
  (if (Variables|Default|GetbIsClosed)
    (CallFunction|OpenDoor)
    (else
      (CallFunction|CloseDoor))))

(fn ConstructionScript)