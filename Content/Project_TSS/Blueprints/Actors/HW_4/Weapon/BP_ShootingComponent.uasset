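; BP_ShootingComponent is a weapon component that spawns projectiles from a muzzle point.
; Fire spawns the current ProjectileClass at the muzzle's world location and rotation.
; SetMuzzlePoint assigns that muzzle, and SelectProjectile switches the class by indexing into AvailableProjectiles without a bounds check.
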(event EventBeginPlay)

(fn Fire
  (bind _muzzlepoint (Variables|Default|GetMuzzlePoint))
  (bind _returnvalue (Transformation|GetWorldTransform _muzzlepoint))
  (Game|SpawnActorfromClass (Variables|Default|GetProjectileClass) (Math|Transform|MakeTransform (.location _returnvalue) (.rotation _returnvalue) "1.000000,1.000000,1.000000") "Undefined" "MultiplyWithRoot" 0 0))

(fn SetMuzzlePoint
  (params (NewMuzzlePoint :type Scene%20Component%20Object%20Reference))
  (Variables|Default|SetMuzzlePoint NewMuzzlePoint))

(fn SelectProjectile
  (params (Index :type Integer))
  (bind _output_get (Variables|Default|SetCurrentProjectileIndex Index))
  (Variables|Default|SetProjectileClass (Utilities|Array|Get(acopy) (Variables|Default|GetAvailableProjectiles) _output_get)))