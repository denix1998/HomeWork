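; BP_DummyTarget is a damageable target dummy actor that shows its health on a text render component.
; TakeHit subtracts the damage amount from Health, clamps the result and destroys the actor when it reaches zero.
; Tick rewrites the displayed text from Health every frame rather than updating it only on hit.
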(event EventTick
  (params (DeltaSeconds :type Float%20%28single-precision%29))
  (Rendering|Components|TextRender|SetText (Variables|Default|GetTextRender) (Utilities|Text|ToText(Float) (Variables|Default|GetHealth) "HalfToEven")))

(fn ConstructionScript)

(fn TakeHit
  (params (DamageAmount :type Float%20%28double-precision%29))
  (Variables|Default|SetHealth (Math|Float|Clamp(Float) (- (Variables|Default|GetHealth) DamageAmount) 0.0 1e+02))
  (if (<= (Variables|Default|GetHealth) 0.0)
    (Actor|DestroyActor)))