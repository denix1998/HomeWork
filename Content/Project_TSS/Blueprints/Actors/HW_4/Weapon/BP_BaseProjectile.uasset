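; BP_BaseProjectile is a base projectile that flies forward and damages dummy targets on impact.
; On BeginPlay it copies its speed variables into the ProjectileMovement component and sets velocity along its local X axis.
; When ProjectileCollision registers a hit, it passes Damage to TakeHit on a BP_DummyTarget, found by casting the hit actor, and destroys itself on any hit.
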(event OnComponentHit(ProjectileCollision)
  (params (HitComponent :type Primitive%20Component%20Object%20Reference) (OtherActor :type Actor%20Object%20Reference) (OtherComp :type Primitive%20Component%20Object%20Reference) (NormalImpulse :type Vector :default "0, 0, 0") (Hit :type Hit%20Result%20Structure%20%28by%20ref%29))
  (bind _asbp_dummy_target (Utilities|Casting|CastToBP_DummyTarget (.HitActor (Collision|BreakHitResult Hit)))
    (:then
      (Default|TakeHit _asbp_dummy_target (Variables|Default|GetDamage))
      (Actor|DestroyActor))
    (:CastFailed
      (Actor|DestroyActor))))

(event EventBeginPlay
  (Variables|/Script/Engine.ProjectileMovementComponent|SetInitialSpeed (Variables|Default|GetProjectileMovement) (Variables|Default|GetInitialSpeed))
  (Variables|/Script/Engine.ProjectileMovementComponent|SetMaxSpeed (Variables|Default|GetProjectileMovement) (Variables|Default|GetMaxSpeed))
  (Game|Components|ProjectileMovement|SetVelocityinLocalSpace (Variables|Default|GetProjectileMovement) (Math|Vector|MakeVector (Variables|Default|GetInitialSpeed) 0.0 0.0)))

(fn ConstructionScript)