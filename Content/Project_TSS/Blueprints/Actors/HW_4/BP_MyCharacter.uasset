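; Player character for a mouse-aimed shooter, moving along world axes via Enhanced Input.
; Each tick, it intersects the cursor ray with a horizontal plane at actor height and turns control yaw toward that point at constant speed.
; A shooting component fires from the muzzle point, with number keys selecting among three projectiles.
; E has two handlers, each sending an interaction message via short forward line traces from muzzle and capsule.
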(event Input|EnhancedActionEvents|EnhancedInputActionIA_Walk
  (params (ActionValue :type Vector%202D%20Structure) (ElapsedSeconds :type Float%20%28double-precision%29) (TriggeredSeconds :type Float%20%28double-precision%29) (InputAction :type Input%20Action%20Object%20Reference :default "/Game/Project_TSS/Blueprints/Input/IA_Walk.IA_Walk"))
  (CallFunction|AddMovement (.x ActionValue) (.y ActionValue)))

(event EventBeginPlay
  (CallFunction|AddMappingContext)
  (bind _asbp_shooting_component (Utilities|Casting|CastToBP_ShootingComponent (Actor|GetComponentbyClass "/Game/Project_TSS/Blueprints/Actors/HW_4/Weapon/BP_ShootingComponent.BP_ShootingComponent_C")))
  (Variables|Default|SetShootingComponent _asbp_shooting_component)
  (Default|SetMuzzlePoint (Variables|Default|GetShootingComponent) (Variables|Default|GetMuzzlePoint)))

(event EventTick
  (params (DeltaSeconds :type Float%20%28single-precision%29))
  (CallFunction|AddMovementRotation))

(event Input|MouseEvents|LeftMouseButton
  (params (Key :type Key%20Structure))
  (:Pressed
    (Default|Fire (Variables|Default|GetShootingComponent))))

(event Input|KeyboardEvents|E
  (params (Key :type Key%20Structure))
  (bind _capsulecomponent (Variables|Collision|GetCapsuleComponent))
  (bind _returnvalue (Transformation|GetWorldLocation _capsulecomponent))
  (:Pressed
    (bind (_outhit _returnvalue_2) (Collision|LineTraceByChannel _returnvalue (+ _returnvalue (* (Math|Vector|GetForwardVector _capsulecomponent) 1e+02)) "TraceTypeQuery1" false 0 "ForDuration"))
    (if _returnvalue_2
      (if (Utilities|DoesObjectImplementInterface (.HitActor (Collision|BreakHitResult _outhit)) "/Game/Project_TSS/Blueprints/Input/BPI_Interface.BPI_Interface_C")
        (Class|BPIInterface|Interface(Message) (.HitActor (Collision|BreakHitResult _outhit)) self)))))

(event Input|KeyboardEvents|E
  (params (Key :type Key%20Structure))
  (:Pressed
    (CallFunction|TryInteract)))

(event Input|KeyboardEvents|1
  (params (Key :type Key%20Structure))
  (:Pressed
    (Default|SelectProjectile (Variables|Default|GetShootingComponent))))

(event Input|KeyboardEvents|2
  (params (Key :type Key%20Structure))
  (:Pressed
    (Default|SelectProjectile (Variables|Default|GetShootingComponent) 1)))

(event Input|KeyboardEvents|3
  (params (Key :type Key%20Structure))
  (:Pressed
    (Default|SelectProjectile (Variables|Default|GetShootingComponent) 2)))

(fn ConstructionScript)

(fn AddMappingContext
  (bind _asplayer_controller (Utilities|Casting|CastToPlayerController (Pawn|GetController)))
  (Input|AddMappingContext (PlayerController|LocalPlayerSubsystems|GetEnhancedInputLocalPlayerSubsystem _asplayer_controller) "/Game/Project_TSS/Blueprints/Input/IMC_UE14Default.IMC_UE14Default" 0 "(bIgnoreAllPressedKeysUntilRelease=True,bForceImmediately=False,bNotifyUserSettings=False)"))

(fn AddMovement
  (params (InputPin :type Float%20%28double-precision%29) (InputPin2 :type Float%20%28double-precision%29))
  (Pawn|Input|AddMovementInput (Math|Vector|GetRightVector "0, 0, 0") InputPin false)
  (Pawn|Input|AddMovementInput (Math|Vector|GetForwardVector "0, 0, 0") InputPin2 false))

(fn AddMovementRotation
  (bind _returnvalue (Game|GetPlayerController 0))
  (bind (_worldlocation _worlddirection) (Game|Player|ConvertMouseLocationToWorldSpace _returnvalue))
  (Pawn|SetControlRotation (Pawn|GetController) (Math|Rotator|MakeRotator 0.0 0.0 (.yaw (Class|KismetMathLibrary|RInterptoConstant (Transformation|GetActorRotation) (Math|Rotator|FindLookatRotation (Transformation|GetActorLocation) (.Intersection (Class|KismetMathLibrary|LinePlaneIntersectionOriginNormal _worldlocation (+ _worldlocation (* _worlddirection 1e+04)) (Transformation|GetActorLocation) "0.000000,0.000000,1.000000"))) (Utilities|Time|GetWorldDeltaSeconds) 7.2e+02)))))

(fn TryInteract
  (bind _muzzlepoint (Variables|Default|GetMuzzlePoint))
  (bind _returnvalue (Transformation|GetWorldLocation _muzzlepoint))
  (bind _outhit (Collision|LineTraceByChannel _returnvalue (+ _returnvalue (* (Math|Vector|GetForwardVector _muzzlepoint) 2e+01)) "TraceTypeQuery1" false 0 "ForDuration"))
  (Class|BPIInteract|Interact(Message) (.HitActor (Collision|BreakHitResult _outhit))))