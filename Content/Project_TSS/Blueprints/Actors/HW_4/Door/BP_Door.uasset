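; BP_Door is an interactable door actor that opens and closes in swing, sliding or lifting style, selected by DoorType.
; Interact toggles IsClose and plays or reverses one timeline, whose alpha lerps DoorPivot's yaw, X location or Z location.
; DoorCollision overlaps show and hide a TextRender for the player character only.
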(event OnComponentBeginOverlap(DoorCollision)
  (params (OverlappedComponent :type Primitive%20Component%20Object%20Reference) (OtherActor :type Actor%20Object%20Reference) (OtherComp :type Primitive%20Component%20Object%20Reference) (OtherBodyIndex :type Integer) (bFromSweep :type Boolean) (SweepResult :type Hit%20Result%20Structure%20%28by%20ref%29))
  (if (== OtherActor (Game|GetPlayerCharacter 0))
    (Rendering|SetVisibility (Variables|Default|GetTextRender) true false)))

(event OnComponentEndOverlap(DoorCollision)
  (params (OverlappedComponent :type Primitive%20Component%20Object%20Reference) (OtherActor :type Actor%20Object%20Reference) (OtherComp :type Primitive%20Component%20Object%20Reference) (OtherBodyIndex :type Integer))
  (if (== OtherActor (Game|GetPlayerCharacter 0))
    (Rendering|SetVisibility (Variables|Default|GetTextRender) false false)))

(event EventInteract
  (if (Variables|Default|GetbIsClose)
    (Variables|Default|SetbIsClose false)
    (bind _alpha (Timeline|TL_DoorAnimation Play)
      (:Update
        (switch Utilities|FlowControl|Switch|SwitchonE_DoorType (Variables|Default|GetDoorType)
          (:NewEnumerator0
            (Transformation|SetRelativeRotation (Variables|Default|GetDoorPivot) (Math|Rotator|MakeRotator 0.0 0.0 (Math|Float|Lerp 0.0 9e+01 _alpha)) false false))
          (:NewEnumerator1
            (Transformation|SetRelativeLocation (Variables|Default|GetDoorPivot) (Math|Vector|MakeVector (Math|Float|Lerp 0.0 1e+02 _alpha) 0.0 0.0) false false))
          (:NewEnumerator2
            (Transformation|SetRelativeLocation (Variables|Default|GetDoorPivot) (Math|Vector|MakeVector 0.0 0.0 (Math|Float|Lerp 0.0 1e+02 _alpha)) false false)))))
    (else
      (Variables|Default|SetbIsClose true)
      (Timeline|TL_DoorAnimation Reverse))))

(fn ConstructionScript)